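; GVR_Pawn is a VR pawn with gaze-dwell and touch interaction, using eye-level tracking and a camera height offset.
; Each Tick, while TraceInteractionComponent hits an actor named TraceInteractiveCube, a counter fills a UIRing progress material on Plane.
; At full count it calls ActiveDown every tick until gaze leaves, which resets the counter.
; Touch press and release call ActiveDown and ActiveUp directly.
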(event `self.ReceiveBeginPlay`
  (`HeadMountedDisplayFunctionLibrary.SetTrackingOrigin` "Eye")
  (`SceneComponent.K2_SetRelativeLocation` (`self.VRCameraRoot`) (`self.Camera Height`) false false))

(event `self.ReceiveTick`
  (params (DeltaSeconds :type "Float (single-precision)"))
  (bind _plane (`self.Plane`))
  (bind _returnvalue (+ (`self.count`) 0.005))
  (if (== "TraceInteractiveCube" (`KismetStringLibrary.Conv_StringToName` (`KismetSystemLibrary.GetDisplayName` (`.HitActor` (`GameplayStatics.BreakHitResult` (`/Game/Blueprints/Components/TraceInteraction-Component.InHit` (`self.TraceInteraction-Component`)))))))
    (if (`KismetMathLibrary.NearlyEqual_FloatFloat` (`self.count`) 1.0 0.0001)
      (`/Game/Blueprints/Components/TraceInteraction-Component.ActiveDown` (`self.TraceInteraction-Component`) self)
      (`PrimitiveComponent.CreateDynamicMaterialInstance` (`self.Plane`) 0 "/Engine/BufferVisualization/AmbientOcclusion.AmbientOcclusion")
      (else
        (`PrimitiveComponent.CreateDynamicMaterialInstance` _plane 0 "/Game/Blueprints/Materials/UIRing.UIRing")
        (`MeshComponent.SetScalarParameterValueOnMaterials` _plane "PercentComplete" _returnvalue)
        (set `self.count` _returnvalue)))
    (else
      (`PrimitiveComponent.CreateDynamicMaterialInstance` (`self.Plane`) 0 "/Engine/BufferVisualization/AmbientOcclusion.AmbientOcclusion")
      (set `self.count` 0.0))))

(event `InputTouch`
  (params (Location :type "Vector Structure") (FingerIndex :type "ETouchIndex Enum"))
  (bind _traceinteraction_component (`self.TraceInteraction-Component`))
  (:`Pressed`
    (`/Game/Blueprints/Components/TraceInteraction-Component.ActiveDown` _traceinteraction_component self))
  (:`Released`
    (`/Game/Blueprints/Components/TraceInteraction-Component.ActiveUp` _traceinteraction_component self)))

(fn `UserConstructionScript`)